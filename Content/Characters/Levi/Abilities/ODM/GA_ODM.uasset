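; Levi's ODM gear gameplay ability, which fires a grapple forward to catch another character.
; Each tick advances paired traces along his forward vector: the sphere catches characters, while the line cancels on walls.
; On a catch, a held key dashes Levi to the target; otherwise the target is pulled in, using root motion forces timed by distance over speed.
; Loose tags mark armor and grabbed states until cleanup.
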(event `self.K2_ActivateAbility`
  ; Init
  (bind _aslevi_class (cast `/Game/Characters/Levi/Levi_Class` (`self.GetAvatarActorFromActorInfo`))
    (:`then`
      (bind _output_get (set `self.Levi` _aslevi_class))
      (set `self.bTargetFound` false)
      (set `self.LastPosition` (`Actor.K2_GetActorLocation` _output_get))
      (`AbilitySystemBlueprintLibrary.AddLooseGameplayTags` (`self.Levi`) (make `GameplayTagContainer` (`|MakeArray` (struct :`TagName` "Character.Status.DoingSomething") (struct :`TagName` "Character.Status.ParryArmor") (struct :`TagName` "Character.Status.HyperArmor") (struct :`TagName` "Character.Ability.Active") :!type "GameplayTag Structure")) true)
      (set `self.bTargetFound` false)
      (set `self.Target` null)
      (set `self.bGrappling` true)
      (`AbilityTask_PlayMontageAndWait.CreatePlayMontageAndWaitProxy` "None" "/Game/Characters/Levi/Anims/Levi_ODM_Idle_Montage.Levi_ODM_Idle_Montage"))
    (:`CastFailed`
      (`self.K2_CancelAbility`))))

(event `self.OnTickEvent`
  (params (DeltaSeconds :type "Float (single-precision)"))
  (bind _lastposition (`self.LastPosition`))
  (bind _array (`|MakeArray` (`self.Levi`) :!type "Actor Object Reference"))
  (bind _returnvalue (+ _lastposition (* DeltaSeconds (`self.GrappleSpeed`) (`Actor.GetActorForwardVector` (`self.Levi`)))))
  ; Grapple Connecting
  (if (`self.bGrappling`)
    (bind _outhit (`KismetSystemLibrary.SphereTraceSingleByProfile` _lastposition _returnvalue 15.0 "BlockAll" false _array "Persistent"))
    (bind (_outhit_2 _returnvalue_2) (`KismetSystemLibrary.LineTraceSingleByProfile` _lastposition _returnvalue "BlockAll" false _array "Persistent"))
    (set `self.LastPosition` _returnvalue)
    (bind (_bblockinghit _binitialoverlap _time _distance _location _impactpoint _normal _impactnormal _physmat _hitactor) (`GameplayStatics.BreakHitResult` _outhit))
    (if _bblockinghit
      (bind _asjfcharacter (cast `JFCharacter` _hitactor)
        (:`then`
          (set `self.Target` _asjfcharacter)
          (set `self.bTargetFound` true)
          (set `self.bGrappling` false)
          (`self.PostGrapple`))
        (:`CastFailed`
          (if _returnvalue_2
            (`KismetSystemLibrary.PrintString` "ODM Ability Canceled - Wire Hit Wall" true true (struct :`R` 1.0 :`A` 1.0) 30.0)
            (`self.K2_EndAbility`)))))))

(event `PostGrapple`
  ; Grab Type Selection
  (`/Engine/EditorBlueprintResources/StandardMacros.IsValid` (`self.Target`)
    (:`Is Valid`
      (`AbilitySystemBlueprintLibrary.AddLooseGameplayTags` (`self.Target`) (make `GameplayTagContainer` (`|MakeArray` (struct :`TagName` "Character.Status.Grabbed") :!type "GameplayTag Structure")) true)
      (if (`self.isKeyHeld`)
        (`self.Go To Target`)
        (else
          (`self.Pull Target`))))
    (:`Is Not Valid`
      (`self.K2_EndAbility`))))

(event `Go To Target`
  ; Dash to Target
  (`AbilityTask_PlayMontageAndWait.CreatePlayMontageAndWaitProxy` "None" "/Game/Characters/Levi/Anims/Levi_ODM_Dash_Montage.Levi_ODM_Dash_Montage"
    (:`then`
      (`AbilityTask_ApplyRootMotionConstantForce.ApplyRootMotionConstantForce` "None" (`Actor.GetActorForwardVector` (`self.Levi`)) (`self.DashSpeed`) (/ (`.Distance` (`self.GetDashLocation`)) (`self.DashSpeed`)) false null "SetVelocity"
        (:`OnFinish`
          (`self.K2_EndAbility`))))))

(event `Pull Target`
  (bind _target (`self.Target`))
  (bind (_returnvalue_roll _returnvalue_pitch) (`KismetMathLibrary.BreakRotator` (`Actor.K2_GetActorRotation` _target)))
  (bind (_returnvalue_roll_2 _returnvalue_pitch_2 _returnvalue_yaw) (`KismetMathLibrary.BreakRotator` (`KismetMathLibrary.FindLookAtRotation` (`Actor.K2_GetActorLocation` _target) (`Actor.K2_GetActorLocation` (`self.Levi`)))))
  ; Pull Target
  (`AbilityTask_PlayMontageAndWaitWithNotify.CreatePlayMontageAndWaitWithNotifyProxy` "None" "/Game/Characters/Levi/Anims/Levi_ODM_Pull_Montage.Levi_ODM_Pull_Montage" 1.0 "None" true 1.0 0.0 false (`self.Target`)
    (:`then`
      (`Actor.K2_SetActorRotation` _target (`KismetMathLibrary.MakeRotator` _returnvalue_roll _returnvalue_pitch _returnvalue_yaw) false)
      (`AbilityTask_ApplyRootMotionConstantForceOnActor.ApplyRootMotionConstantForceOnActor` "None" (* (`Actor.GetActorForwardVector` (`self.Levi`)) -1.0) (`self.PullSpeed`) (/ (`.Distance` (`self.GetPullLocation`)) (`self.PullSpeed`)) false null "MaintainLastRootMotionVelocity" (0.0 0.0 0.0) 0.0 false (`self.Target`)
        (:`OnFinish`
          (`self.K2_EndAbility`))))))

(event `self.K2_OnEndAbility`
  (params (bWasCancelled :type Boolean))
  (bind _target (`self.Target`))
  ; Ability Cleanup
  (`self.MontageStop` -1.0)
  (set `self.bTargetFound` false)
  (set `self.bGrappling` false)
  (`/Engine/EditorBlueprintResources/StandardMacros.IsValid` _target
    (:`Is Valid`
      (`Character.StopAnimMontage` _target null)
      (`AbilitySystemBlueprintLibrary.RemoveLooseGameplayTags` _target (make `GameplayTagContainer` (`|MakeArray` (struct :`TagName` "Character.Status.Grabbed") :!type "GameplayTag Structure")) true))
    (:`Is Not Valid`
      _))
  (set `self.Target` null)
  (`AbilitySystemBlueprintLibrary.RemoveLooseGameplayTags` (`self.Levi`) (make `GameplayTagContainer` (`|MakeArray` (struct :`TagName` "Character.Status.DoingSomething") (struct :`TagName` "Character.Status.ParryArmor") (struct :`TagName` "Character.Status.HyperArmor") (struct :`TagName` "Character.Ability.Active") :!type "GameplayTag Structure")) true))
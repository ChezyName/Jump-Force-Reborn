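; Levi's dash AOE gameplay ability, a forward dash with a multi-hit capsule hitbox attached to the character.
; A montage notify enables the hitbox, adds the Judgement Dash cue, hides the mesh and starts a curve-driven root motion force for a set duration.
; A close enough hit swaps that force for a post-hit one, while tick periodically resets hit actors for repeat hits.
; Ending restores visibility and clears status tags and cue.
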(event `self.K2_ActivateAbility`
  (bind _returnvalue (`self.GetCharacter`))
  (bind _returnvalue_2 (`self.GetCharacter`))
  (`/Engine/EditorBlueprintResources/StandardMacros.IsValid` _returnvalue_2
    (:`Is Valid`
      (`JFCharacter.PlaySoundByWaveAtLocation` _returnvalue_2 "/Game/Characters/Levi/Sounds/ODM_Dash.ODM_Dash" (`Actor.K2_GetActorLocation` _returnvalue_2) (0.75 1.25) (0.75 1.25))
      (`AbilitySystemBlueprintLibrary.AddLooseGameplayTags` (`self.GetCharacter`) (make `GameplayTagContainer` (`|MakeArray` (struct :`TagName` "Character.Status.DoingSomething") (struct :`TagName` "Character.Status.CantLock") (struct :`TagName` "Character.Ability.Active") (struct :`TagName` "Character.Status.NoMeter") :!type "GameplayTag Structure")) true)
      (`JFCharacter.PlaySoundByWave` (`self.GetCharacter`) "/Game/Characters/Levi/Sounds/Levi_Multi_Hit_Dash.Levi_Multi_Hit_Dash" true)
      (bind _returnvalue_3 (`self.CreateHitbox` "Capsule" (0.0 0.0 0.0) (struct) (200.0 200.0 200.0) null (`Character.CapsuleComponent` (`self.GetCharacter`))))
      (set `self.Hitbox` _returnvalue_3)
      (`AbilityTask_PlayMontageAndWaitWithNotify.CreatePlayMontageAndWaitWithNotifyProxy` "None" "/Game/Characters/Levi/Anims/Levi_Dash_Montage.Levi_Dash_Montage" 1.0 "None" true 1.0 0.0 false null
        (:`OnNotifyBegin`
          (`self.EnableHitbox` (`self.Hitbox`))
          (`GameplayCueFunctionLibrary.AddGameplayCueOnActor` _returnvalue (struct :`TagName` "GameplayCue.LeviJudgementDash") (`AbilitySystemBlueprintLibrary.MakeGameplayCueParameters` 0.0))
          (`JFCharacter.setMeshVisibilityServer` _returnvalue false)
          (bind _asynctaskproxy (`AbilityTask_ApplyRootMotionConstantForce.ApplyRootMotionConstantForce` "None" (`Actor.GetActorForwardVector` (`self.GetCharacter`)) (`self.DashStrength`) (`self.DashDuration`) false "/Game/Characters/Levi/Abilities/DashAOE/LeviDashCurve.LeviDashCurve" "SetVelocity")
            (:`then`
              (set `self.DashTask` _asynctaskproxy)
              (`KismetSystemLibrary.Delay` (`self.DashDuration`))
              (`self.K2_EndAbility`))))))))

(event `self.OnHitboxHit`
  (params (Hitbox :type "Hitbox Object Reference") (TargetHit :type "Actor Object Reference"))
  (bind _dashtask (`self.DashTask`))
  (`/Engine/EditorBlueprintResources/StandardMacros.IsValid` _dashtask
    (:`Is Valid`
      (`/Engine/EditorBlueprintResources/StandardMacros.IsValid` TargetHit
        (:`Is Valid`
          (if (<= (`KismetMathLibrary.Vector_Distance` (`Actor.K2_GetActorLocation` TargetHit) (`Actor.K2_GetActorLocation` (`self.GetCharacter`))) (`self.DashStopDistance`))
            (`GameplayTask.EndTask` _dashtask)
            (`AbilityTask_ApplyRootMotionConstantForce.ApplyRootMotionConstantForce` "None" (`Actor.GetActorForwardVector` (`self.GetCharacter`)) (`self.DashStrengthPostHit`) (`self.DashDuration`) false null "SetVelocity")))))))

(event `self.K2_OnEndAbility`
  (params (bWasCancelled :type Boolean))
  (bind _returnvalue (`self.GetCharacter`))
  (`/Engine/EditorBlueprintResources/StandardMacros.IsValid` _returnvalue
    (:`Is Valid`
      (`JFCharacter.setMeshVisibilityServer` _returnvalue true)
      (`AbilitySystemBlueprintLibrary.RemoveLooseGameplayTags` (`self.GetCharacter`) (make `GameplayTagContainer` (`|MakeArray` (struct :`TagName` "Character.Status.DoingSomething") (struct :`TagName` "Character.Status.CantLock") (struct :`TagName` "Character.Ability.Active") (struct :`TagName` "Character.Status.NoMeter") :!type "GameplayTag Structure")) true)
      (`GameplayCueFunctionLibrary.RemoveGameplayCueOnActor` (`self.GetCharacter`) (struct :`TagName` "GameplayCue.LeviJudgementDash") (`AbilitySystemBlueprintLibrary.MakeGameplayCueParameters` 0.0)))))

(event `self.OnTickEvent`
  (params (DeltaSeconds :type "Float (single-precision)"))
  (bind _output_get (set `self.fDamagePerSecondDelay` (- (`self.fDamagePerSecondDelay`) DeltaSeconds)))
  (if (<= _output_get 0.0)
    (`self.ResetActorsHit`)
    (set `self.fDamagePerSecondDelay` (`self.DamagePerSecondDelay`))))
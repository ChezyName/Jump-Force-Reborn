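; Levi's Judgement Cut End gameplay ability: he vanishes and damages a large area around him while time is stopped.
; A dash montage notify stops time through JFGameState (or cancels if already stopped), enables a capsule hitbox, adds the cue and hides the mesh.
; Tick periodically clears the hit-actor list so damage repeats.
; Timed delays disable the hitbox, then restore visibility and time; replicated loose tags mark the ability until it ends.
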(event `self.K2_ActivateAbility`
  (bind _returnvalue (`self.GetCharacter`))
  (bind _gs (`self.GS`))
  (`/Engine/EditorBlueprintResources/StandardMacros.IsValid` (`self.GetCharacter`)
    (:`Is Valid`
      (bind _asjfgame_state (cast `JFGameState` (`GameplayStatics.GetGameState`))
        (:`then`
          (set `self.GS` _asjfgame_state)
          (`AbilitySystemBlueprintLibrary.AddLooseGameplayTags` (`self.GetCharacter`) (make `GameplayTagContainer` (`|MakeArray` (struct :`TagName` "Character.Status.DoingSomething") (struct :`TagName` "Character.Status.CantLock") (struct :`TagName` "Character.Ability.Active") :!type "GameplayTag Structure")) true)
          (bind _returnvalue_2 (`self.CreateHitbox` "Capsule" (0.0 0.0 0.0) (struct) (600.0 600.0 600.0) null (`Character.CapsuleComponent` (`self.GetCharacter`))))
          (set `self.Hitbox` _returnvalue_2)
          (`AbilityTask_PlayMontageAndWaitWithNotify.CreatePlayMontageAndWaitWithNotifyProxy` "None" "/Game/Characters/Levi/Anims/Levi_Dash_Montage.Levi_Dash_Montage" 1.0 "None" true 1.0 0.0 false null
            (:`OnNotifyBegin`
              (if (`JFGameState.IsTimeStopped` _gs)
                (`self.K2_CancelAbility`)
                (else
                  (`JFGameState.StopTime` _gs (`self.GetCharacter`))
                  (`self.EnableHitbox` (`self.Hitbox`))
                  (`GameplayCueFunctionLibrary.AddGameplayCueOnActor` _returnvalue (struct :`TagName` "GameplayCue.JCE") (`AbilitySystemBlueprintLibrary.MakeGameplayCueParameters` 0.0))
                  (`JFCharacter.setMeshVisibilityServer` _returnvalue false)
                  (`KismetSystemLibrary.Delay` (`self.TS Time`))
                  (`self.DisableHitbox` (`self.Hitbox`))
                  (`GameplayCueFunctionLibrary.RemoveGameplayCueOnActor` (`self.GetCharacter`) (struct :`TagName` "GameplayCue.JCE") (`AbilitySystemBlueprintLibrary.MakeGameplayCueParameters` 0.0))
                  (`KismetSystemLibrary.Delay` (`self.TS End Lag`))
                  (`JFCharacter.setMeshVisibilityServer` (`self.GetCharacter`) true)
                  (`JFGameState.ResumeTime` (`self.GS`))
                  (`self.K2_EndAbility`))))))
        (:`CastFailed`
          (`self.K2_CancelAbility` :!label _label))))
    (:`Is Not Valid`
      (goto _label))))

(event `self.K2_OnEndAbility`
  (params (bWasCancelled :type Boolean))
  (`AbilitySystemBlueprintLibrary.RemoveLooseGameplayTags` (`self.GetCharacter`) (make `GameplayTagContainer` (`|MakeArray` (struct :`TagName` "Character.Status.DoingSomething") (struct :`TagName` "Character.Status.CantLock") (struct :`TagName` "Character.Ability.Active") :!type "GameplayTag Structure")) true)
  (`GameplayCueFunctionLibrary.RemoveGameplayCueOnActor` (`self.GetCharacter`) (struct :`TagName` "GameplayCue.JCE") (`AbilitySystemBlueprintLibrary.MakeGameplayCueParameters` 0.0)))

(event `self.OnTickEvent`
  (params (DeltaSeconds :type "Float (single-precision)"))
  (bind _output_get (set `self.fDamagePerSecondDelay` (- (`self.fDamagePerSecondDelay`) DeltaSeconds)))
  (if (<= _output_get 0.0)
    (`self.ResetActorsHit`)
    (set `self.fDamagePerSecondDelay` (`self.DamagePerSecondDelay`))))
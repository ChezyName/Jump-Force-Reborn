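; DIO's Blood Suck grab ability, which drains health from a caught character and heals DIO.
; An init montage opens a hitbox during its notify window; a hit turns the victim toward DIO, tags them Grabbed and disables collision between them.
; Paired montages then play, with a notify window enabling per-tick damage and matching healing, followed by a final hit.
; Ending the ability removes tags and restores collision.
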(event `self.K2_ActivateAbility`
  (bind _returnvalue (`self.GetFirstActorHit`))
  (bind _hitbox (`self.Hitbox`))
  (bind _char (`self.Char`))
  (bind _char_2 (`self.Char`))
  (bind _targethit (`self.TargetHit`))
  (bind _char_3 (`self.Char`))
  (bind _targethit_2 (`self.TargetHit`))
  (bind _targethit_3 (`self.TargetHit`))
  (bind (_returnvalue_roll _returnvalue_pitch) (`KismetMathLibrary.BreakRotator` (`Actor.K2_GetActorRotation` _targethit_3)))
  (bind _returnvalue_2 (`SceneComponent.GetSocketLocation` (`Character.Mesh` _char) "hand_R"))
  (bind (_returnvalue_roll_2 _returnvalue_pitch_2 _returnvalue_yaw) (`KismetMathLibrary.BreakRotator` (`KismetMathLibrary.FindLookAtRotation` (`Actor.K2_GetActorLocation` _targethit_3) (`Actor.K2_GetActorLocation` (`self.Char`)))))
  (set `self.Damage` (`self.DamageBase`))
  (set `self.AbilityHit` false)
  (set `self.TargetHit` null)
  (bind _asdio (cast `/Game/Characters/DIO/DIO` (`self.GetAvatarActorFromActorInfo`))
    (:`then`
      (bind _output_get (set `self.Char` _asdio))
      (`JFCharacter.PlaySoundByWaveAtLocation` _output_get "/Game/Characters/DIO/Sounds/Blood_Suck_Start_Sound.Blood_Suck_Start_Sound" (`Actor.K2_GetActorLocation` (`self.Char`)) (0.75 1.25) (0.75 1.25))
      (`AbilitySystemBlueprintLibrary.AddLooseGameplayTags` _output_get (make `GameplayTagContainer` (`|MakeArray` (struct :`TagName` "Character.Status.DoingSomething") (struct :`TagName` "Character.Ability") (struct :`TagName` "Character.Status.CantLock") :!type "GameplayTag Structure")) true)
      (bind _returnvalue_3 (`self.CreateHitbox` "Box" (0.0 120.0 -70.0) (struct) (32.0 32.0 32.0) (`Character.Mesh` (`self.Char`)) "root" -1.0 true))
      (set `self.Hitbox` _returnvalue_3)
      (`AbilityTask_PlayMontageAndWaitWithNotify.CreatePlayMontageAndWaitWithNotifyProxy` "None" "/Game/Characters/DIO/Anims/Blood_Suck_Init_Montage.Blood_Suck_Init_Montage" 1.0 "None" true 1.0 0.0 false null
        (:`then`
          (`JFCharacter.PlaySoundByWave` (`self.Char`) "/Game/Characters/DIO/Sounds/DIO_WRYYY.DIO_WRYYY" true))
        (:`OnNotifyBegin`
          (`self.EnableHitbox` _hitbox))
        (:`OnNotifyEnd`
          (`self.DisableHitbox` _hitbox)
          (`/Engine/EditorBlueprintResources/StandardMacros.IsValid` _returnvalue
            (:`Is Valid`
              (bind _asjfcharacter (cast `JFCharacter` _returnvalue))
              (set `self.TargetHit` _asjfcharacter)
              (set `self.AbilityHit` true)
              (`self.DestroyHitbox` (`self.Hitbox`))
              (`self.MontageStop` -1.0)
              (`PrimitiveComponent.IgnoreActorWhenMoving` (`Character.CapsuleComponent` _targethit) _char_3 true)
              (`PrimitiveComponent.IgnoreActorWhenMoving` (`Character.Mesh` _targethit) _char_3 true)
              (`Actor.K2_SetActorRotation` _targethit_2 (`KismetMathLibrary.MakeRotator` _returnvalue_roll _returnvalue_pitch _returnvalue_yaw) false)
              (`AbilitySystemBlueprintLibrary.AddLooseGameplayTags` _targethit_2 (make `GameplayTagContainer` (`|MakeArray` (struct :`TagName` "Character.Status.Grabbed") :!type "GameplayTag Structure")) true)
              (`AbilityTask_PlayMontageAndWaitWithNotify.CreatePlayMontageAndWaitWithNotifyProxy` "None" "/Game/Characters/DIO/Anims/Blood_Suck_Recv_Montage.Blood_Suck_Recv_Montage" 1.0 "None" true 1.0 0.0 false (`self.TargetHit`)
                (:`then`
                  (`AbilityTask_PlayMontageAndWaitWithNotify.CreatePlayMontageAndWaitWithNotifyProxy` "None" "/Game/Characters/DIO/Anims/BloodSuck_AM.BloodSuck_AM" 1.0 "None" true 1.0 0.0 false null
                    (:`OnNotifyBegin`
                      (set `self.isHealing` true)
                      (`JFCharacter.PlaySoundByWaveAtLocation` _char "/Game/Characters/DIO/Sounds/Blood_Suck_1.Blood_Suck_1" _returnvalue_2 (0.75 1.25) (0.75 1.25))
                      (`KismetSystemLibrary.Delay` 0.2)
                      (`JFCharacter.PlaySoundByWaveAtLocation` _char "/Game/Characters/DIO/Sounds/Blood_Suck_2.Blood_Suck_2" _returnvalue_2 (0.75 1.25) (0.75 1.25)))
                    (:`OnNotifyEnd`
                      (set `self.isHealing` false)
                      (`JFCharacter.TakeDamage` (`self.TargetHit`) (`self.DamageFinal`) _char_2 true)
                      (`JFCharacter.PlaySoundByType` _char_2 "LightHit" true))
                    (:`OnBlendOut`
                      (set `self.isHealing` false)
                      (`self.K2_EndAbility`))))))))
        (:`OnBlendOut`
          (if (not (`self.AbilityHit`))
            (`self.K2_EndAbility`)))))
    (:`CastFailed`
      (`self.K2_CancelAbility`))))

(event `self.OnHitboxHit`
  (params (Hitbox :type "Hitbox Object Reference"))
  (bind _returnvalue_location (`KismetMathLibrary.BreakTransform` (`Hitbox.GetWorldTransform` Hitbox)))
  (bind _char (`self.Char`))
  (`/Engine/EditorBlueprintResources/StandardMacros.IsValid` _char
    (:`Is Valid`
      (`JFCharacter.PlaySoundByWaveAtLocation` _char "/Game/Characters/DIO/Sounds/TW_Heavy_Punch.TW_Heavy_Punch" _returnvalue_location (0.75 1.25) (0.75 1.25)))))

(event `self.K2_OnEndAbility`
  (params (bWasCancelled :type Boolean))
  (bind _char (`self.Char`))
  (bind _char_2 (`self.Char`))
  (bind _targethit (`self.TargetHit`))
  (`/Engine/EditorBlueprintResources/StandardMacros.IsValid` _char_2
    (:`Is Valid`
      (`AbilitySystemBlueprintLibrary.RemoveLooseGameplayTags` _char_2 (make `GameplayTagContainer` (`|MakeArray` (struct :`TagName` "Character.Status.DoingSomething") (struct :`TagName` "Character.Ability") (struct :`TagName` "Character.Status.CantLock") :!type "GameplayTag Structure")) true)
      (`/Engine/EditorBlueprintResources/StandardMacros.IsValid` (`self.TargetHit`)
        (:`Is Valid`
          (`AbilitySystemBlueprintLibrary.RemoveLooseGameplayTags` (`self.TargetHit`) (make `GameplayTagContainer` (`|MakeArray` (struct :`TagName` "Character.Status.Grabbed") :!type "GameplayTag Structure")) true)
          (`PrimitiveComponent.IgnoreActorWhenMoving` (`Character.CapsuleComponent` _targethit) _char false)
          (`PrimitiveComponent.IgnoreActorWhenMoving` (`Character.Mesh` _targethit) _char false))))))

(event `self.OnTickEvent`
  (params (DeltaSeconds :type "Float (single-precision)"))
  (bind _targethit (`self.TargetHit`))
  (bind _char (`self.Char`))
  (`/Engine/EditorBlueprintResources/StandardMacros.IsValid` (`self.Char`)
    (:`Is Valid`
      (`/Engine/EditorBlueprintResources/StandardMacros.IsValid` _targethit
        (:`Is Valid`
          (if (`self.isHealing`)
            (`JFCharacter.TakeDamage` _targethit (* DeltaSeconds (`self.DamagePerHeal`)) _char true)
            (`JFCharacter.HealPlayer` _char (* DeltaSeconds (`self.DamagePerHeal`)))))))))
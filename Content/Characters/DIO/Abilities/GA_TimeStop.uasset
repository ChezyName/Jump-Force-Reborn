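; DIO's Time Stop gameplay ability, which freezes time through JFGameState and can only activate while time is not already stopped.
; It applies replicated busy tags, positions The World stand relative to DIO, and plays the ZaWurdo montage on both.
; A montage notify calls StopTime and ends the ability, removing tags and stand, with ResumeTime placed after a TimestopDuration delay that follows EndAbility.
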(event `self.K2_ActivateAbility`
  (bind _theworld (`/Game/Characters/DIO/DIO.TheWorld` (`self.Char`)))
  (bind _asjfgame_state (cast `JFGameState` (`GameplayStatics.GetGameState`))
    (:`then`
      (bind _output_get (set `self.GS` _asjfgame_state))
      (if (`JFGameState.IsTimeStopped` _output_get)
        (`self.K2_EndAbility`)
        (else
          (bind _asdio (cast `/Game/Characters/DIO/DIO` (`self.GetAvatarActorFromActorInfo`))
            (:`then`
              (bind _output_get_2 (set `self.Char` _asdio))
              (`AbilitySystemBlueprintLibrary.AddLooseGameplayTags` _output_get_2 (make `GameplayTagContainer` (`|MakeArray` (struct :`TagName` "Character.Status.DoingSomething") (struct :`TagName` "Character.Ability") :!type "GameplayTag Structure")) true)
              (`KismetSystemLibrary.PrintString` "Time Stopping" true true (struct :`R` 1.0 :`A` 1.0))
              (if (`JFGameState.IsTimeStopped` (`self.GS`))
                (`self.K2_EndAbility`)
                (else
                  (`/Game/Characters/DIO/TheWorld.ActivateStand` _theworld false)
                  (`Actor.K2_SetActorTransform` _theworld (`KismetMathLibrary.MakeTransform` (`KismetMathLibrary.TransformLocation` (`Actor.GetTransform` (`self.Char`)) (`self.StandLocationTS`)) (`Actor.K2_GetActorRotation` (`self.Char`))) false false)
                  (`AbilityTask_PlayMontageAndWaitWithNotify.CreatePlayMontageAndWaitWithNotifyProxy` "None" "/Game/Characters/DIO/Anims/ZaWurdo_AM.ZaWurdo_AM" 1.0 "None" true 1.0 0.0 false (`/Game/Characters/DIO/DIO.TheWorld` (`self.Char`))
                    (:`then`
                      (`AbilityTask_PlayMontageAndWaitWithNotify.CreatePlayMontageAndWaitWithNotifyProxy` "None" "/Game/Characters/DIO/Anims/ZaWurdo_AM.ZaWurdo_AM" 1.0 "None" true 1.0 0.0 false null
                        (:`OnNotifyBegin`
                          (if (`JFGameState.IsTimeStopped` (`self.GS`))
                            (`self.K2_EndAbility` :!label _label)
                            (else
                              (`JFGameState.StopTime` (`self.GS`) (`self.Char`))
                              (`self.K2_EndAbility`)
                              (`KismetSystemLibrary.Delay` (`self.TimestopDuration`))
                              (`JFGameState.ResumeTime` (`self.GS`)))))
                        (:`OnCompleted`
                          (goto _label))
                        (:`OnBlendOut`
                          (goto _label))
                        (:`OnInterrupted`
                          (goto _label))
                        (:`OnCancelled`
                          (goto _label))))))))
            (:`CastFailed`
              (`self.K2_CancelAbility`))))))
    (:`CastFailed`
      (`self.K2_EndAbility`))))

(event `self.K2_OnEndAbility`
  (params (bWasCancelled :type Boolean))
  (bind _char (`self.Char`))
  (`/Engine/EditorBlueprintResources/StandardMacros.IsValid` _char
    (:`Is Valid`
      (`AbilitySystemBlueprintLibrary.RemoveLooseGameplayTags` _char (make `GameplayTagContainer` (`|MakeArray` (struct :`TagName` "Character.Status.DoingSomething") (struct :`TagName` "Character.Ability") :!type "GameplayTag Structure")) true)
      (`/Game/Characters/DIO/TheWorld.DisableStand` (`/Game/Characters/DIO/DIO.TheWorld` (`self.Char`)) 0.0)
      (set `self.Char` null))))

(fn `K2_CanActivateAbility`
  (params (ActorInfo :type "GameplayAbilityActorInfo Structure") (Handle :type "GameplayAbilitySpecHandle Structure"))
  (returns (RelevantTags :type "GameplayTagContainer Structure") (ReturnValue :type Boolean))
  (bind _asjfgame_state (cast `JFGameState` (`GameplayStatics.GetGameState`))
    (:`then`
      (return (struct) (not (`JFGameState.IsTimeStopped` _asjfgame_state))))
    (:`CastFailed`
      (return (struct) false))))
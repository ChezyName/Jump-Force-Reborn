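; Broly's Ki Blast gameplay ability, a channeled barrage that spawns blasts repeatedly while the key is held.
; Activation applies blocking tags, montage and gameplay cue, then after a short delay enables per-second meter use and starts firing until release.
; Blasts scatter randomly within a forward cone sized by lock-on state, homing on the locked target or spreading only in yaw without one.
; Ending the ability removes the tags and cue and stops the montage.
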(event `self.K2_ActivateAbility`
  (`AbilitySystemBlueprintLibrary.AddLooseGameplayTags` (`self.GetCharacter`) (make `GameplayTagContainer` (`|MakeArray` (struct :`TagName` "Character.Ability.Active") (struct :`TagName` "Character.Status.CantMove") (struct :`TagName` "Character.Status.DoingSomething") (struct :`TagName` "Character.Status.NoMeter") :!type "GameplayTag Structure")) true)
  (`AbilityTask_PlayMontageAndWaitWithNotify.CreatePlayMontageAndWaitWithNotifyProxy` "None" "/Game/Characters/Broly/Anims/Broly_KI_Blast_Loop_Montage.Broly_KI_Blast_Loop_Montage" 1.0 "None" false 1.0 0.0 false null
    (:`then`
      (`GameplayCueFunctionLibrary.AddGameplayCueOnActor` (`self.GetCharacter`) (struct :`TagName` "GameplayCue.Broly.KI_Blast") (`AbilitySystemBlueprintLibrary.MakeGameplayCueParameters` 0.0))
      (`KismetSystemLibrary.Delay` 0.5)
      (set `self.TakesMeterPerSecond` true)
      (if (`self.isKeyHeld`) :!label _label
        (`self.Toss KI`)
        (`KismetSystemLibrary.Delay` 0.05)
        (goto _label)
        (else
          (`KismetSystemLibrary.Delay` 0.15)
          (`self.K2_EndAbility`))))))

(event `self.K2_OnEndAbility`
  (params (bWasCancelled :type Boolean))
  (bind _returnvalue (`self.GetCharacter`))
  (`AbilitySystemBlueprintLibrary.RemoveLooseGameplayTags` _returnvalue (make `GameplayTagContainer` (`|MakeArray` (struct :`TagName` "Character.Ability.Active") (struct :`TagName` "Character.Status.CantMove") (struct :`TagName` "Character.Status.DoingSomething") (struct :`TagName` "Character.Status.NoMeter") :!type "GameplayTag Structure")) true)
  (`GameplayCueFunctionLibrary.RemoveGameplayCueOnActor` _returnvalue (struct :`TagName` "GameplayCue.Broly.KI_Blast") (`AbilitySystemBlueprintLibrary.MakeGameplayCueParameters` 0.0 0.0 (struct) (struct) (struct) (struct) (struct) (`self.KISpawnLoc`)))
  (`self.MontageStop` -1.0))

(event `Toss KI`
  (bind _returnvalue (`self.GetCharacter`))
  (bind _returnvalue_2 (`self.GetCharacter`))
  (bind _returnvalue_3 (`KismetMathLibrary.RandomUnitVectorInConeInDegrees` (`Actor.GetActorForwardVector` (`self.GetCharacter`)) (`KismetMathLibrary.SelectFloat` (`self.ConeAngleLockedOn`) (`self.ConeAngleNotLocked`) (`JFCharacter.isLockedOn` (`self.GetCharacter`)))))
  (bind (_returnvalue_roll _returnvalue_pitch _returnvalue_yaw) (`KismetMathLibrary.BreakRotator` (`KismetMathLibrary.MakeRotFromX` _returnvalue_3)))
  ; Toss a Ki blast with Psudo Rando Rotation
  (bind _returnvalue_4 (`|SpawnActorFromClass` "/Game/Characters/Broly/Abilities/KI-Blast/KiBlast.KiBlast_C" (`KismetMathLibrary.MakeTransform` (`KismetMathLibrary.TransformLocation` (`SceneComponent.K2_GetComponentToWorld` (`Character.Mesh` (`self.GetCharacter`))) (`self.KISpawnLoc`)) (`KismetMathLibrary.SelectRotator` (`KismetMathLibrary.MakeRotFromX` _returnvalue_3) (`KismetMathLibrary.MakeRotator` 0.0 0.0 _returnvalue_yaw) (`JFCharacter.isLockedOn` (`self.GetCharacter`)))) "AlwaysSpawn" "MultiplyWithRoot" _returnvalue _returnvalue))
  (`PrimitiveComponent.IgnoreActorWhenMoving` (`/Game/Characters/Broly/Abilities/KI-Blast/KiBlast.Box` _returnvalue_4) (`self.GetCharacter`) true)
  (if (`JFCharacter.isLockedOn` _returnvalue_2)
    (`/Game/Characters/Broly/Abilities/KI-Blast/KiBlast.LockOnTarget` _returnvalue_4 (`JFCharacter.LockOnCharacter` _returnvalue_2))))
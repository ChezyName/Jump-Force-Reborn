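; Gameplay ability for Broly's Ki Dash, a hyper-armored forward charge that explodes on the first character it hits.
; An init montage with ki cues leads into the dash montage, which enables a mesh-attached hitbox for a limited duration.
; While dashing, tick uses a countdown to periodically reapply curve-driven root motion force along the facing direction.
; A character hit deals damage and ends the ability, clearing tags, cues and hitbox.
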(event `self.K2_ActivateAbility`
  ; Begin / Init
  (`AbilitySystemBlueprintLibrary.AddLooseGameplayTags` (`self.GetCharacter`) (make `GameplayTagContainer` (`|MakeArray` (struct :`TagName` "Character.Ability.Active") (struct :`TagName` "Character.Status.DoingSomething") (struct :`TagName` "Character.Status.HyperArmor") :!type "GameplayTag Structure")) true)
  (set `self.ForceEndOnMeterZero` false)
  (set `self.EndAbilityOnKeyRelease` false)
  (`self.Dash_Init`)
  (bind _returnvalue (`self.CreateHitbox` "Box" (50.0 0.0 180.0) (struct) (100.0 100.0 100.0) null (`Character.Mesh` (`self.GetCharacter`))))
  (set `self.Hitbox` _returnvalue))

(event `self.OnHitboxHit`
  (params (Hitbox :type "Hitbox Object Reference") (TargetHit :type "Actor Object Reference"))
  (bind _asjfcharacter (cast `JFCharacter` TargetHit))
  (`GameplayCueFunctionLibrary.ExecuteGameplayCueOnActor` _asjfcharacter (struct :`TagName` "GameplayCue.Broly.KI_Explode") (`AbilitySystemBlueprintLibrary.MakeGameplayCueParameters` 0.0))
  (set `self.isDashing` false)
  (`JFCharacter.TakeDamage` _asjfcharacter (`self.ExplosionDamage`) (`self.GetCharacter`) true false null)
  (`self.K2_EndAbility`))

(event `self.OnTickEvent`
  (params (DeltaSeconds :type "Float (single-precision)"))
  ; Tick
  (if (`self.isDashing`)
    (bind _output_get (set `self.fDashDelay` (- (`self.fDashDelay`) DeltaSeconds)))
    (if (<= _output_get 0.0)
      (`AbilityTask_ApplyRootMotionConstantForce.ApplyRootMotionConstantForce` "None" (`Actor.GetActorForwardVector` (`self.GetCharacter`)) (`self.DashStrength`) (`self.DashDelay`) true "/Game/Characters/_Core/_Dash/DashCurve.DashCurve" "MaintainLastRootMotionVelocity"
        (:`then`
          (set `self.fDashDelay` (`self.DashDelay`)))))))

(event `DashPart`
  ; Dashing
  (`AbilityTask_PlayMontageAndWait.CreatePlayMontageAndWaitProxy` "None" "/Game/Characters/Broly/Anims/Broly_Dash_Montage.Broly_Dash_Montage"
    (:`then`
      (`self.EnableHitbox` (`self.Hitbox`))
      (`self.K2_AddGameplayCue` (struct :`TagName` "GameplayCue.Broly.KI_Dash") (struct) false)
      (set `self.isDashing` true)
      (`AbilitySystemBlueprintLibrary.AddLooseGameplayTags` (`self.GetCharacter`) (make `GameplayTagContainer` (`|MakeArray` (struct :`TagName` "Character.Status.CantLock") :!type "GameplayTag Structure")) true)
      (`KismetSystemLibrary.Delay` (`self.DashDuration`))
      (if (`self.isDashing`)
        (`self.DisableHitbox` (`self.Hitbox`))
        (set `self.isDashing` false)
        (`self.K2_EndAbility`)))))

(event `self.K2_OnEndAbility`
  (params (bWasCancelled :type Boolean))
  ; End Ability
  (set `self.isDashing` false)
  (`AbilitySystemBlueprintLibrary.RemoveLooseGameplayTags` (`self.GetCharacter`) (make `GameplayTagContainer` (`|MakeArray` (struct :`TagName` "Character.Ability.Active") (struct :`TagName` "Character.Status.DoingSomething") (struct :`TagName` "Character.Status.HyperArmor") (struct :`TagName` "Character.Status.CantLock") :!type "GameplayTag Structure")) true)
  (`self.MontageStop` -1.0)
  (`self.K2_RemoveGameplayCue` (struct :`TagName` "GameplayCue.Broly.KI_Dash"))
  (`self.K2_RemoveGameplayCue` (struct :`TagName` "GameplayCue.Broly.KI_Dash_Balls"))
  (`self.DestroyHitbox` (`self.Hitbox`)))

(event `Dash_Init`
  ; Setup Dash
  (`AbilityTask_PlayMontageAndWaitWithNotify.CreatePlayMontageAndWaitWithNotifyProxy` "None" "/Game/Characters/Broly/Anims/Broly_Dash_Init_Montage.Broly_Dash_Init_Montage" 1.0 "None" true 1.0 0.0 false null
    (:`then`
      (`self.K2_AddGameplayCue` (struct :`TagName` "GameplayCue.Broly.KI_Dash_Init") (struct) false))
    (:`OnNotifyBegin`
      (`self.K2_AddGameplayCue` (struct :`TagName` "GameplayCue.Broly.KI_Dash_Balls") (struct) false))
    (:`OnCompleted`
      (`self.K2_RemoveGameplayCue` (struct :`TagName` "GameplayCue.Broly.KI_Dash_Init"))
      (`self.DashPart`))))
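; Broly's Ki Grab gameplay ability: a hyper-armored grab that leads into a damaging Ki dash.
; An init montage's notify window enables a root-attached hitbox, and the ability ends on blend-out if nothing is caught.
; A hit tags the victim as Grabbed, snaps it into place and plays paired receive and dash montages.
; A near-per-tick delay loop applies hitstun-free damage under a dash cue until the dash completes.
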(event `self.OnHitboxHit`
  (params (Hitbox :type "Hitbox Object Reference") (TargetHit :type "Actor Object Reference"))
  ; Hitbox
  (set `self.TargetHit` false)
  (bind _asjfcharacter (cast `JFCharacter` TargetHit))
  (set `self.Target` _asjfcharacter)
  (`self.MontageStop` -1.0)
  (`self.PostInit`))

(event `self.K2_ActivateAbility`
  (bind _hitbox (`self.Hitbox`))
  ; Init
  (`self.Init`)
  (`AbilitySystemBlueprintLibrary.AddLooseGameplayTags` (`self.GetCharacter`) (make `GameplayTagContainer` (`|MakeArray` (struct :`TagName` "Character.Ability.Active") (struct :`TagName` "Character.Status.DoingSomething") (struct :`TagName` "Character.Status.HyperArmor") :!type "GameplayTag Structure")) true)
  (bind _returnvalue (`self.CreateHitbox` "Box" (0.0 128.0 -48.0) (struct) (50.0 18.0 18.0) null (`Character.Mesh` (`self.GetCharacter`)) "root"))
  (set `self.Hitbox` _returnvalue)
  (`AbilityTask_PlayMontageAndWaitWithNotify.CreatePlayMontageAndWaitWithNotifyProxy` "None" "/Game/Characters/Broly/Anims/Broly_Grab_Init_Montage.Broly_Grab_Init_Montage" 1.0 "None" true 1.0 0.0 false null
    (:`OnNotifyBegin`
      (`self.EnableHitbox` _hitbox))
    (:`OnNotifyEnd`
      (`self.DisableHitbox` _hitbox))
    (:`OnBlendOut`
      (if (not (`self.TargetHit`))
        (`/Engine/EditorBlueprintResources/StandardMacros.IsValid` (`self.Target`)
          (:`Is Not Valid`
            (`self.K2_EndAbility`)))))))

(event `Init`
  ; Small Inits
  (set `self.TargetHit` false)
  (set `self.TargetTakesDMG` false))

(event `PostInit`
  (bind _returnvalue (`self.GetCharacter`))
  (bind (_returnvalue_roll _returnvalue_pitch _returnvalue_yaw) (`KismetMathLibrary.BreakRotator` (`Actor.K2_GetActorRotation` (`self.GetCharacter`))))
  ; Post Init Grab Animations
  (`AbilitySystemBlueprintLibrary.AddLooseGameplayTags` (`self.Target`) (make `GameplayTagContainer` (`|MakeArray` (struct :`TagName` "Character.Status.Grabbed") :!type "GameplayTag Structure")) true)
  (`Actor.K2_SetActorLocationAndRotation` (`self.Target`) (+ (* (`Actor.GetActorForwardVector` _returnvalue) (`self.DistanceTeleportForGrab`)) (`Actor.K2_GetActorLocation` _returnvalue)) (`KismetMathLibrary.MakeRotator` _returnvalue_roll _returnvalue_pitch _returnvalue_yaw) false false)
  (`AbilityTask_PlayMontageAndWaitWithNotify.CreatePlayMontageAndWaitWithNotifyProxy` "None" "/Game/Characters/Broly/Anims/Broly_Grab_Recv_Montage.Broly_Grab_Recv_Montage" 1.0 "None" false 1.0 0.0 false (`self.Target`)
    (:`then`
      (`AbilityTask_PlayMontageAndWaitWithNotify.CreatePlayMontageAndWaitWithNotifyProxy` "None" "/Game/Characters/Broly/Anims/Broly_Grab_Dash_Montage.Broly_Grab_Dash_Montage" 1.0 "None" false 1.0 0.0 false null
        (:`then`
          (`self.TargetTakeDamage`)
          (`self.K2_AddGameplayCue` (struct :`TagName` "GameplayCue.Broly.KI_Dash")))
        (:`OnCompleted`
          (set `self.TargetTakesDMG` false)
          (`self.K2_EndAbility`))))))

(event `TargetTakeDamage`
  (bind _target (`self.Target`))
  ; Grab Damage Loop
  (set `self.TargetTakesDMG` true)
  (if (`self.TargetTakesDMG`) :!label _label
    (`/Engine/EditorBlueprintResources/StandardMacros.IsValid` _target
      (:`Is Valid`
        (`JFCharacter.TakeDamage` _target (`self.DashDamage`) (`self.GetCharacter`) true false null)
        (`KismetSystemLibrary.Delay` 0.0001)
        (goto _label)))))

(event `self.K2_OnEndAbility`
  (params (bWasCancelled :type Boolean))
  (bind _target (`self.Target`))
  ; Ability End
  (`AbilitySystemBlueprintLibrary.RemoveLooseGameplayTags` (`self.GetCharacter`) (make `GameplayTagContainer` (`|MakeArray` (struct :`TagName` "Character.Ability.Active") (struct :`TagName` "Character.Status.DoingSomething") (struct :`TagName` "Character.Status.HyperArmor") :!type "GameplayTag Structure")) true)
  (`/Engine/EditorBlueprintResources/StandardMacros.IsValid` _target
    (:`Is Valid`
      (`AbilitySystemBlueprintLibrary.RemoveLooseGameplayTags` _target (make `GameplayTagContainer` (`|MakeArray` (struct :`TagName` "Character.Status.Grabbed") :!type "GameplayTag Structure")) true)
      (set `self.Target` null)
      (`self.DestroyHitbox` (`self.Hitbox`)))))